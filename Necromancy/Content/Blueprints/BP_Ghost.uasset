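; BP_Ghost is a ghost actor that the player completes by touching it once its villager condition and a score limit are met.
; On capsule overlap it scans its Villagers, setting Completed when all are dead or Zombie-tagged, or when it hits any invalid entry.
; If the game mode's Score exceeds ScoreLimit, completion activates the linked checkpoint's next step and destroys the ghost.
; ChangeMaterial applies one material to both hands and the capsule.
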(event `CompleteGhost`
  (bind _checkpoint (`self.CheckPoint`))
  (`/Engine/EditorBlueprintResources/StandardMacros.IsValid` _checkpoint
    (:`Is Valid`
      (bind _asbp_checkpoint (cast `/Game/Blueprints/BP_Checkpoint` _checkpoint))
      (`/Game/Blueprints/BP_Checkpoint.ActivateNext` _asbp_checkpoint))
    (:`Is Not Valid`
      _))
  (`self.K2_DestroyActor`))

(event `self.CapsuleComponent.OnComponentBeginOverlap`
  (params (OverlappedComponent :type "PrimitiveComponent Object Reference") (OtherActor :type "Actor Object Reference") (OtherComp :type "PrimitiveComponent Object Reference") (OtherBodyIndex :type Integer) (bFromSweep :type Boolean) (SweepResult :type "HitResult Structure (by ref)"))
  (cast `/Game/Blueprints/BP_PlayerCharacter` OtherActor)
  (`self.CheckActorsDeath`)
  (if (`self.Completed`)
    (bind _asbp_my_game_mode (cast `/Game/Blueprints/BP_MyGameMode` (`GameplayStatics.GetGameMode`)))
    (if (> (`/Game/Blueprints/BP_MyGameMode.Score` _asbp_my_game_mode) (`self.ScoreLimit`))
      (`self.CompleteGhost`))))

(event `CheckActorsDeath`
  (for _array_element (`self.Villagers`)
    (`/Engine/EditorBlueprintResources/StandardMacros.IsValid` _array_element
      (:`Is Valid`
        (bind _asbp_villager (cast `/Game/Blueprints/BP_Villager` _array_element))
        (if (or (`/Game/Blueprints/BPC_Health.IsDead` (`/Game/Blueprints/BP_BaseCharacter.BPC_Health` _asbp_villager)) (`self.ActorHasTag` _asbp_villager "Zombie"))
          (set `self.IsDead` true)
          (else
            (set `self.IsDead` false)
            (break))))
      (:`Is Not Valid`
        (set `self.Completed` true :!label _label))))
  (if (`self.IsDead`)
    (goto _label)))

(fn `ChangeMaterial`
  (params (Material :type "MaterialInstance Object Reference"))
  (`PrimitiveComponent.SetMaterial` (`self.RightHand`) 0 Material)
  (`PrimitiveComponent.SetMaterial` (`self.LeftHand`) 0 Material)
  (`PrimitiveComponent.SetMaterial` (`self.Capsule`) 0 Material))

(fn `UserConstructionScript`)