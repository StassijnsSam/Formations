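; AI controller for a zombie pawn that follows the player, moves to a position or attacks an enemy.
; A looping half-second timer runs Behavior, which switches on CurrentBehaviorType and reissues the matching AI MoveTo, with no behavior tree.
; The attack branch fires CallAttack as soon as the move toward Enemy is issued, without waiting for arrival.
; The behavior type, destination and enemy are only read here.
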(event `self.ReceiveBeginPlay`
  (`KismetSystemLibrary.K2_SetTimer` null "Behavior" 0.5 true))

(event `Behavior`
  (switch `string` (`self.CurrentBehaviorType`)
    (:`Follow`
      (`|AIMoveTo` (`self.K2_GetPawn`) (0.0 0.0 0.0) (`GameplayStatics.GetPlayerCharacter` 0) 200.0))
    (:`MoveToPos`
      (`|AIMoveTo` (`self.K2_GetPawn`) (`self.MoveTo`) null 10.0 true))
    (:`AttackOnPos`
      (`|AIMoveTo` (`self.K2_GetPawn`) (0.0 0.0 0.0) (`self.Enemy`) 5.0 true
        (:`then`
          (`self.Attack`))))))

(fn `UserConstructionScript`)