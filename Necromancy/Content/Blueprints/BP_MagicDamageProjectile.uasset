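; BP_MagicDamageProjectile is a homing magic projectile that damages its assigned target.
; On BeginPlay it copies its damage from the player controller's MagicDamage value.
; SetHomingTarget stores the target and steers ProjectileMovement toward that actor's capsule component.
; Its sphere reacts only to overlapping that target, applying damage through a BP_BaseCharacter's health component before destroying itself.
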(event `self.ReceiveBeginPlay`
  (bind _asbp_my_player_controller (cast `/Game/Blueprints/BP_MyPlayerController` (`GameplayStatics.GetPlayerController` 0)))
  (set `self.DamageAmount` (`/Game/Blueprints/BP_MyPlayerController.MagicDamage` _asbp_my_player_controller)))

(event `SetHomingTarget`
  (params (HomingTarget :type "Actor Object Reference"))
  (bind _returnvalue (`self.GetComponentByClass` HomingTarget "/Script/Engine.CapsuleComponent"))
  (bind _projectilemovement (`self.ProjectileMovement`))
  (set `self.HomingTarget` HomingTarget)
  (`/Engine/EditorBlueprintResources/StandardMacros.IsValid` _returnvalue
    (:`Is Valid`
      (set `ProjectileMovementComponent.HomingTargetComponent` _returnvalue _projectilemovement)
      (set `ProjectileMovementComponent.bIsHomingProjectile` true _projectilemovement))))

(event `self.Sphere.OnComponentBeginOverlap`
  (params (OverlappedComponent :type "PrimitiveComponent Object Reference") (OtherActor :type "Actor Object Reference") (OtherComp :type "PrimitiveComponent Object Reference") (OtherBodyIndex :type Integer) (bFromSweep :type Boolean) (SweepResult :type "HitResult Structure (by ref)"))
  (if (== OtherActor (`self.HomingTarget`))
    (bind _asbp_base_character (cast `/Game/Blueprints/BP_BaseCharacter` (`self.HomingTarget`)))
    (`/Game/Blueprints/BPC_Health.Do Damage` (`/Game/Blueprints/BP_BaseCharacter.BPC_Health` _asbp_base_character) (`self.DamageAmount`))
    (`self.K2_DestroyActor`)))

(fn `UserConstructionScript`)