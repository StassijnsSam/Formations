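; Armed villager Blueprint that extends its parent's behavior with a weapon held in a socket component.
; On BeginPlay, unless the villager is flagged dead from start, it spawns an actor of WeaponClass and snaps it to WeaponSocket.
; When the health component fires OnDead, the weapon detaches in world space and its static mesh starts simulating physics, so it drops.
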(event `self.BPC_Health.OnDead`
  (bind _currentweapon (`self.CurrentWeapon`))
  (`/Engine/EditorBlueprintResources/StandardMacros.IsValid` _currentweapon
    (:`Is Valid`
      (`self.K2_DetachFromActor` _currentweapon "KeepWorld" "KeepWorld" "KeepRelative")
      (`PrimitiveComponent.SetSimulatePhysics` (`/Game/Blueprints/BP_Spear.StaticMesh` _currentweapon) true))))

(event `self.ReceiveBeginPlay`
  (bind _weaponsocket (`self.WeaponSocket`))
  (`parent.ReceiveBeginPlay`)
  (if (not (`self.isDeadFromStart`))
    (bind _returnvalue (`|SpawnActorFromClass` (`self.WeaponClass`) (`SceneComponent.K2_GetComponentToWorld` _weaponsocket) "Undefined" "OverrideRootScale" null null))
    (bind _output_get (set `self.CurrentWeapon` _returnvalue))
    (`self.K2_AttachToComponent` _output_get _weaponsocket "None" "SnapToTarget" "SnapToTarget" "KeepRelative" true)))

(fn `UserConstructionScript`
  (`parent.UserConstructionScript`))