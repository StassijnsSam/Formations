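; BPC_Highlight is an actor component that toggles a highlight on its owning actor.
; EnableHighlight and DisableHighlight loop over every valid StaticMeshComponent on the owner and switch Render Custom Depth on or off.
; It only writes the meshes into the custom depth buffer; the visible highlight effect is not defined here.
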(event `EnableHighlight`
  (for _array_element (`Actor.K2_GetComponentsByClass` (`self.GetOwner`) "/Script/Engine.StaticMeshComponent")
    (`/Engine/EditorBlueprintResources/StandardMacros.IsValid` _array_element
      (:`Is Valid`
        (`PrimitiveComponent.SetRenderCustomDepth` _array_element true)))))

(event `DisableHighlight`
  (for _array_element (`Actor.K2_GetComponentsByClass` (`self.GetOwner`) "/Script/Engine.StaticMeshComponent")
    (`/Engine/EditorBlueprintResources/StandardMacros.IsValid` _array_element
      (:`Is Valid`
        (`PrimitiveComponent.SetRenderCustomDepth` _array_element false)))))