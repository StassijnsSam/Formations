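; AI controller for villagers that runs the BT_Villager behavior tree on possess and records the pawn's starting location in the Blackboard.
; Successfully sensing an actor tagged Friendly or Zombie stores it as EnemyActor, sets HasLineOfSight and cancels the forget timer.
; Any other perception update starts a LineOfSightTimer-length delay, after which the line-of-sight flag and enemy are cleared.
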(event `self.AIPerception.OnTargetPerceptionUpdated`
  (params (Actor :type "Actor Object Reference") (Stimulus :type "AIStimulus Structure"))
  (bind _blackboard (`self.Blackboard`))
  (if (and (or (`self.ActorHasTag` Actor "Friendly") (`self.ActorHasTag` Actor "Zombie")) (`.bSuccessfullySensed` (break `AIStimulus` Stimulus)))
    (`KismetSystemLibrary.K2_ClearAndInvalidateTimerHandle` (`self.EnemyTimer`))
    (`BlackboardComponent.SetValueAsBool` _blackboard (`self.HasLineOfSight`) true)
    (`BlackboardComponent.SetValueAsObject` _blackboard (`self.EnemyActor`) Actor)
    (else
      (bind _returnvalue (`KismetSystemLibrary.K2_SetTimerDelegate` (delegate `StartEnemyTimer`) (`self.LineOfSightTimer`)))
      (set `self.EnemyTimer` _returnvalue))))

(event `StartEnemyTimer`
  (bind _blackboard (`self.Blackboard`))
  (`BlackboardComponent.SetValueAsBool` _blackboard (`self.HasLineOfSight`) false)
  (`BlackboardComponent.SetValueAsObject` _blackboard (`self.EnemyActor`) null))

(event `self.ReceivePossess`
  (params (PossessedPawn :type "Pawn Object Reference"))
  (`self.RunBehaviorTree` "/Game/Blueprints/BT_Villager.BT_Villager")
  (`BlackboardComponent.SetValueAsVector` (`self.Blackboard`) (`self.Start Location`) (`self.K2_GetActorLocation` (`self.K2_GetPawn`))))

(fn `UserConstructionScript`)