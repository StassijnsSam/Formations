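; Player controller for a top-down necromancer game where the player raises dead villagers as zombies and commands them.
; Left click selects and marks a character or ground point, setting selected zombies' AI to follow, attack or move; right mouse feeds the HUD.
; Trade Life spends health on homing damage at enemies or drains zombies to heal.
; It also handles movement, cursor-facing rotation, spring-arm zoom, pausing and spline-drawn formation markers.
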(event `InputAction|DrawFormation`
  (params (Key :type "Key Structure"))
  (:`Pressed`
    ;[1 1 1] Destroy existing splines
    (bind _outactors (`GameplayStatics.GetAllActorsOfClass` "/Script/DemoProject.Spline"))
    (for _array_element _outactors
      (`self.K2_DestroyActor` _array_element))
    (bind _returnvalue (`|SpawnActorFromClass` "/Script/DemoProject.Spline" (`KismetMathLibrary.MakeTransform` (0.0 0.0 0.0)) "Undefined" "OverrideRootScale" null null))
    (`Spline.StartDrawing` _returnvalue))
  (:`Released`
    ;[1 1 1] Stop Drawing
    (bind _outactors_2 (`GameplayStatics.GetAllActorsOfClass` "/Script/DemoProject.Spline"))
    (for _array_element_2 _outactors_2
      (`Spline.StopDrawing` _array_element_2)
      (bind _returnvalue_2 (`Spline.GetPoinstAlongSpline` _array_element_2 8))
      (for _array_element_3 _returnvalue_2
        (`|SpawnActorFromClass` "/Game/Blueprints/BP_MoveTarget.BP_MoveTarget_C" (`KismetMathLibrary.MakeTransform` _array_element_3) "Undefined" "OverrideRootScale" null null)))))

(event `InputAction|Pause`
  (params (Key :type "Key Structure"))
  ;[1 1 1] Cant pause in main menu
  (:`Pressed`
    (bind _returnvalue (`GameplayStatics.GetCurrentLevelName` true))
    (if (not (`KismetStringLibrary.EqualEqual_StrStr` _returnvalue "MainMenuLevel"))
      (`/Engine/EditorBlueprintResources/StandardMacros.IsValid` (`self.PauseScreen`)
        (:`Is Valid`
          _)
        (:`Is Not Valid`
          (bind _returnvalue_2 (`|CreateWidget` "/Game/UI/BPW_PauseScreen.BPW_PauseScreen_C"))
          (set `self.PauseScreen` _returnvalue_2)))
      (`UserWidget.AddToViewport` (`self.PauseScreen`) 0)
      (`GameplayStatics.SetGamePaused` true))))

(event `InputAction|ZoomIn`
  (params (Key :type "Key Structure"))
  (:`Pressed`
    (bind _asbp_player_character (cast `/Game/Blueprints/BP_PlayerCharacter` (`GameplayStatics.GetPlayerPawn` 0)))
    (bind _springarm (`/Game/Blueprints/BP_PlayerCharacter.SpringArm` _asbp_player_character))
    (bind _returnvalue (- (`SpringArmComponent.TargetArmLength` _springarm) 5.0))
    (if (> _returnvalue (`self.MinArmLength`))
      (set `SpringArmComponent.TargetArmLength` _returnvalue _springarm)
      (bind (_returnvalue_roll _returnvalue_pitch _returnvalue_yaw) (`KismetMathLibrary.BreakRotator` (`SpringArmComponent.GetTargetRotation` _springarm)))
      (bind _returnvalue_2 (+ _returnvalue_pitch 2.0))
      (if (< _returnvalue_2 -40.0)
        (`SceneComponent.K2_SetRelativeRotation` _springarm (`KismetMathLibrary.MakeRotator` _returnvalue_roll _returnvalue_2 _returnvalue_yaw) false false)))))

(event `InputAction|ZoomOut`
  (params (Key :type "Key Structure"))
  (:`Pressed`
    (bind _asbp_player_character (cast `/Game/Blueprints/BP_PlayerCharacter` (`GameplayStatics.GetPlayerPawn` 0)))
    (bind _springarm (`/Game/Blueprints/BP_PlayerCharacter.SpringArm` _asbp_player_character))
    (bind _returnvalue (+ (`SpringArmComponent.TargetArmLength` _springarm) 5.0))
    (if (< _returnvalue (`self.MaxArmLength`))
      (set `SpringArmComponent.TargetArmLength` _returnvalue _springarm)
      (bind (_returnvalue_roll _returnvalue_pitch _returnvalue_yaw) (`KismetMathLibrary.BreakRotator` (`SpringArmComponent.GetTargetRotation` _springarm)))
      (bind _returnvalue_2 (- _returnvalue_pitch 2.0))
      (if (> _returnvalue_2 -90.0)
        (`SceneComponent.K2_SetRelativeRotation` _springarm (`KismetMathLibrary.MakeRotator` _returnvalue_roll _returnvalue_2 _returnvalue_yaw) false false)))))

(event `self.ReceiveTick`
  (params (DeltaSeconds :type "Float (single-precision)"))
  (if (`self.RightMousePressed`)
    (bind _asbp_hud (cast `/Game/UI/BP_HUD` (`self.GetHUD`)))
    (`/Game/UI/BP_HUD.Event Held` _asbp_hud)))

(event `Key|RightMouseButton`
  (params (Key :type "Key Structure"))
  (bind _returnvalue (`self.GetHUD`))
  (:`Pressed`
    (set `self.RightMousePressed` true)
    (bind _asbp_hud (cast `/Game/UI/BP_HUD` _returnvalue))
    (`/Game/UI/BP_HUD.Event Pressed` _asbp_hud))
  (:`Released`
    (set `self.RightMousePressed` false)
    (bind _asbp_hud_2 (cast `/Game/UI/BP_HUD` _returnvalue))
    (`/Game/UI/BP_HUD.Event Released` _asbp_hud_2)))

(event `InputAction|TradeLife`
  (params (Key :type "Key Structure"))
  (bind _clickedactor (`self.ClickedActor`))
  (bind _clickedactor_2 (`self.ClickedActor`))
  (:`Pressed`
    (`/Engine/EditorBlueprintResources/StandardMacros.IsValid` _clickedactor
      (:`Is Valid`
        (`|ExecutionSequence`
          (:`then_0`
            (if (`self.ActorHasTag` _clickedactor "Enemy")
              (bind _asbp_player_character (cast `/Game/Blueprints/BP_PlayerCharacter` (`GameplayStatics.GetPlayerPawn` 0)))
              (if (> (`/Game/Blueprints/BPC_Health.CurrentHealth` (`/Game/Blueprints/BP_BaseCharacter.BPC_Health` _asbp_player_character)) (`self.TradeDamage`))
                (cast `/Game/Blueprints/BP_Villager` _clickedactor_2)
                (bind _asbp_player_character_2 (cast `/Game/Blueprints/BP_PlayerCharacter` (`GameplayStatics.GetPlayerPawn` 0)))
                (`/Game/Blueprints/BPC_Health.Do Damage` (`/Game/Blueprints/BP_BaseCharacter.BPC_Health` _asbp_player_character_2) (`self.TradeDamage`))
                (bind _returnvalue (`|SpawnActorFromClass` "/Game/Blueprints/BP_MagicDamageProjectile.BP_MagicDamageProjectile_C" (`self.GetTransform` (`GameplayStatics.GetPlayerPawn` 0)) "AlwaysSpawn" "OverrideRootScale" null null))
                (`/Game/Blueprints/BP_MagicDamageProjectile.SetHomingTarget` _returnvalue _clickedactor_2))))
          (:`then_1`
            (if (`self.ActorHasTag` _clickedactor "Zombie")
              (bind _asbp_player_character_3 (cast `/Game/Blueprints/BP_PlayerCharacter` (`GameplayStatics.GetPlayerPawn` 0)))
              (bind _bpc_health (`/Game/Blueprints/BP_BaseCharacter.BPC_Health` _asbp_player_character_3))
              (if (< (`/Game/Blueprints/BPC_Health.CurrentHealth` _bpc_health) (`/Game/Blueprints/BPC_Health.MaxHealth` _bpc_health))
                (bind _asbp_villager (cast `/Game/Blueprints/BP_Villager` (`self.ClickedActor`)))
                (bind _returnvalue_2 (`|SpawnActorFromClass` "/Game/Blueprints/BP_MagicHealProjectile.BP_MagicHealProjectile_C" (`self.GetTransform` _asbp_villager) "AlwaysSpawn" "OverrideRootScale" null null))
                (`/Game/Blueprints/BP_MagicDamageProjectile.SetHomingTarget` _returnvalue_2 (`GameplayStatics.GetPlayerPawn` 0))
                (`/Game/Blueprints/BPC_Health.Do Damage` (`/Game/Blueprints/BP_BaseCharacter.BPC_Health` _asbp_villager) 100.0)))))))))

(event `InputAction|RaiseUndead`
  (params (Key :type "Key Structure"))
  (bind _returnvalue (`self.K2_GetActorLocation` (`self.K2_GetPawn`)))
  (:`Pressed`
    (bind _outactors (`KismetSystemLibrary.SphereOverlapActors` _returnvalue (`self.MagicRadius`) (`|MakeArray` "ObjectTypeQuery3" :!type "EObjectTypeQuery Enum")))
    (`GameplayStatics.SpawnEmitterAtLocation` "/Game/Particles/P_RaiseUndead.P_RaiseUndead" (- _returnvalue (0.0 0.0 10.0)))
    (`KismetSystemLibrary.Delay` 1.0)
    (for _array_element _outactors
      (bind _asbp_villager (cast `/Game/Blueprints/BP_Villager` _array_element))
      (`/Engine/EditorBlueprintResources/StandardMacros.IsValid` _asbp_villager
        (:`Is Valid`
          (if (`/Game/Blueprints/BPC_Health.IsDead` (`/Game/Blueprints/BP_BaseCharacter.BPC_Health` _asbp_villager))
            (`/Game/Blueprints/BP_Villager.Raise` _asbp_villager)
            ;[1 1 1] Make it so raised zombies are selected from the start
            (`KismetArrayLibrary.Array_AddUnique` (`self.SelectedZombies`) _array_element)
            (`/Game/Blueprints/BPC_Highlight.EnableHighlight` (`/Game/Blueprints/BP_BaseCharacter.BPC_Highlight` _asbp_villager))))))))

(event `Key|LeftMouseButton`
  (params (Key :type "Key Structure"))
  (bind (_hitresult _returnvalue) (`self.GetHitResultUnderCursorByChannel` "TraceTypeQuery2"))
  (bind _clickedactor (`self.ClickedActor`))
  (bind _clickedactor_2 (`self.ClickedActor`))
  (bind _movetoflag (`self.MoveToFlag`))
  (bind (_bblockinghit _binitialoverlap _time _distance _location _impactpoint _normal _impactnormal _physmat _hitactor) (`GameplayStatics.BreakHitResult` _hitresult))
  (:`Pressed`
    (if _returnvalue
      (`|ExecutionSequence`
        (:`then_0`
          ;[1 1 1] Deselect the old one
          (`/Engine/EditorBlueprintResources/StandardMacros.IsValid` _clickedactor
            (:`Is Valid`
              (bind _asbp_base_character (cast `/Game/Blueprints/BP_BaseCharacter` _clickedactor)
                (:`then`
                  (for _array_element (`self.GetAttachedActors` _asbp_base_character true)
                    (bind _asbp_move_target (cast `/Game/Blueprints/BP_MoveTarget` _array_element))
                    (`self.K2_DetachFromActor` _asbp_move_target "KeepRelative" "KeepRelative" "KeepRelative")
                    (`self.K2_DestroyActor` _asbp_move_target))
                  ;[1 1 1] If it is another actor select it, if it is the same do nothing (leave it unselected)
                  (if (== _hitactor (`self.ClickedActor`))
                    (set `self.ClickedActor` null :!label _label)
                    (else
                      (`/Engine/EditorBlueprintResources/StandardMacros.IsValid` _hitactor :!label _label_2
                        (:`Is Valid`
                          (cast `/Game/Blueprints/BP_BaseCharacter` _hitactor
                            (:`then`
                              (bind _output_get (set `self.ClickedActor` _hitactor))
                              (bind _returnvalue_2 (`self.GetTransform` _output_get))
                              (bind _returnvalue_3 (`|SpawnActorFromClass` "/Game/Blueprints/BP_MoveTarget.BP_MoveTarget_C" (`KismetMathLibrary.MakeTransform` (`KismetMathLibrary.MakeVector` (.x (.location _returnvalue_2)) (.y (.location _returnvalue_2)) (+ (.z (.location _returnvalue_2)) 75.0)) (.rotation _returnvalue_2) (.scale _returnvalue_2)) "AlwaysSpawn" "OverrideRootScale" null null))
                              (`self.K2_AttachToActor` _returnvalue_3 _output_get "None" "KeepWorld" "SnapToTarget" "KeepRelative" true))
                            (:`CastFailed`
                              (goto _label))))
                        (:`Is Not Valid`
                          (goto _label))))))
                (:`CastFailed`
                  (goto _label))))
            (:`Is Not Valid`
              (goto _label_2))))
        (:`then_1`
          (`/Engine/EditorBlueprintResources/StandardMacros.IsValid` _movetoflag
            (:`Is Valid`
              (`self.K2_DestroyActor` _movetoflag))
            (:`Is Not Valid`
              _))
          (`/Engine/EditorBlueprintResources/StandardMacros.IsValid` _clickedactor_2
            (:`Is Valid`
              (`self.MoveZombiesToActor` _clickedactor_2))
            (:`Is Not Valid`
              (bind _returnvalue_4 (`|SpawnActorFromClass` "/Game/Blueprints/BP_MoveTarget.BP_MoveTarget_C" (`KismetMathLibrary.Conv_VectorToTransform` _location) "Undefined" "OverrideRootScale" null null))
              (set `self.MoveToFlag` _returnvalue_4)
              (`self.MoveZombiesToLocation` _location))))))))

(event `InputAxis|MovementForward`
  (params (AxisValue :type "Float (single-precision)"))
  (bind _returnvalue (`self.K2_GetPawn`))
  ;[1 1 1] Handle Movement Input
  (`/Engine/EditorBlueprintResources/StandardMacros.IsValid` _returnvalue
    (:`Is Valid`
      (`Pawn.AddMovementInput` _returnvalue (1.0 0.0 0.0) AxisValue false))))

(event `InputAxis|MovementRight`
  (params (AxisValue :type "Float (single-precision)"))
  (bind _returnvalue (`self.K2_GetPawn`))
  ;[1 1 1] Handle Movement Input
  (`/Engine/EditorBlueprintResources/StandardMacros.IsValid` _returnvalue
    (:`Is Valid`
      (`Pawn.AddMovementInput` _returnvalue (0.0 1.0 0.0) AxisValue false))))

(event `InputAxis|LookUp`
  (params (AxisValue :type "Float (single-precision)"))
  ;[1 1 1] Controller Rotation
  (bind _returnvalue (`KismetMathLibrary.MakeVector` AxisValue (stale `InputAxis|LookRight` AxisValue)))
  (if (> (`KismetMathLibrary.VSize` _returnvalue) 0.25) :!label _label_3
    (`self.SetControlRotation` (`KismetMathLibrary.Conv_VectorToRotator` _returnvalue))))

(event `InputAxis|LookRight`
  (params (AxisValue :type "Float (single-precision)"))
  ;[1 1 1] Controller Rotation
  (goto _label_3))

(event `InputAxisKey|MouseX`
  (params (AxisValue :type "Float (single-precision)"))
  (bind (_hitresult _returnvalue) (`self.GetHitResultUnderCursorByChannel` "TraceTypeQuery1"))
  (bind (_returnvalue_roll _returnvalue_pitch _returnvalue_yaw) (`KismetMathLibrary.BreakRotator` (`KismetMathLibrary.FindLookAtRotation` (`self.K2_GetActorLocation` (`self.K2_GetPawn`)) (`.Location` (`GameplayStatics.BreakHitResult` _hitresult)))))
  ;[1 1 1] Mouse Rotation
  (if (> (`KismetMathLibrary.VSize` (`KismetMathLibrary.MakeVector` AxisValue (stale `InputAxisKey|MouseY` AxisValue))) 0.25) :!label _label_4
    (if _returnvalue
      (`self.SetControlRotation` (`KismetMathLibrary.MakeRotator` 0.0 0.0 _returnvalue_yaw)))))

(event `InputAxisKey|MouseY`
  (params (AxisValue :type "Float (single-precision)"))
  ;[1 1 1] Mouse Rotation
  (goto _label_4))

(fn `MoveZombiesToActor`
  (params (TargetActor :type "Actor Object Reference"))
  (for _array_element (`self.SelectedZombies`)
    (`/Engine/EditorBlueprintResources/StandardMacros.IsValid` _array_element
      (:`Is Valid`
        (bind _asbp_zombie_aicontroller (cast `/Game/Blueprints/BP_ZombieAIController` (`AIBlueprintHelperLibrary.GetAIController` _array_element)))
        (if (== TargetActor (`GameplayStatics.GetPlayerPawn` 0))
          ;[1 1 1] If you clicked on player follow it
          (set `/Game/Blueprints/BP_ZombieAIController.CurrentBehaviorType` "Follow" _asbp_zombie_aicontroller)
          (else
            ;[1 1 1] If you clicked on an enemy attack it
            (set `/Game/Blueprints/BP_ZombieAIController.CurrentBehaviorType` "AttackOnPos" _asbp_zombie_aicontroller)
            (set `/Game/Blueprints/BP_ZombieAIController.Enemy` TargetActor _asbp_zombie_aicontroller)))))))

(fn `MoveZombiesToLocation`
  (params (Location :type "Vector Structure"))
  (for _array_element (`self.SelectedZombies`)
    (`/Engine/EditorBlueprintResources/StandardMacros.IsValid` _array_element
      (:`Is Valid`
        (bind _asbp_zombie_aicontroller (cast `/Game/Blueprints/BP_ZombieAIController` (`AIBlueprintHelperLibrary.GetAIController` _array_element)))
        ;[1 1 1] If you clicked on a location make them move to it
        (set `/Game/Blueprints/BP_ZombieAIController.CurrentBehaviorType` "MoveToPos" _asbp_zombie_aicontroller)
        (set `/Game/Blueprints/BP_ZombieAIController.MoveTo` Location _asbp_zombie_aicontroller)))))

(fn `UserConstructionScript`)