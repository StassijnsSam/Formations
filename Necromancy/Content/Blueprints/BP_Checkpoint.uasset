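; Tutorial checkpoint actor that triggers a linked ghost's timed dialogue when the player enters it.
; A looping timer steps through text lines on the ghost's widget, then marks villager-less ghosts completed.
; When the player leaves, completed auto-disappear ghosts receive CompleteGhost.
; ActivateNext chains checkpoints by enabling the next, revealing its ghost and retargeting the tutorial arrow, or opens Level01 at the finish.
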(event `UpdateText`
  (`self.SetText`)
  (if (< (+ (`self.CurrentIndex`) 1) (`KismetArrayLibrary.Array_Length` (`self.TextArray`)))
    (set `self.CurrentIndex` (+ (`self.CurrentIndex`) 1))
    (else
      (`KismetSystemLibrary.K2_ClearTimer` null "UpdateText")
      (bind _asbp_ghost (cast `/Game/Blueprints/BP_Ghost` (`self.Ghost`)))
      (`/Engine/EditorBlueprintResources/StandardMacros.IsValid` _asbp_ghost
        (:`Is Valid`
          (if (== (`KismetArrayLibrary.Array_Length` (`/Game/Blueprints/BP_Ghost.Villagers` _asbp_ghost)) 0)
            (set `/Game/Blueprints/BP_Ghost.Completed` true _asbp_ghost)))))))

(event `self.ReceiveActorBeginOverlap`
  (params (OtherActor :type "Actor Object Reference"))
  (bind _ghost (`self.Ghost`))
  (cast `/Game/Blueprints/BP_PlayerCharacter` OtherActor)
  (if (`self.CanStart`)
    (set `self.CanStart` false)
    (`/Engine/EditorBlueprintResources/StandardMacros.IsValid` _ghost
      (:`Is Valid`
        (`self.SetActorHiddenInGame` _ghost false)
        (`self.SetText`)
        (if (< (`self.CurrentIndex`) (`KismetArrayLibrary.Array_Length` (`self.TextArray`)))
          (set `self.CurrentIndex` (+ (`self.CurrentIndex`) 1))
          (`KismetSystemLibrary.K2_SetTimerDelegate` (delegate `UpdateText`) (`self.TextDelay`) true))))))

(event `ActivateNext`
  (bind _nextcheckpoint (`self.NextCheckPoint`))
  (if (`self.IsFinishLevel`)
    (`GameplayStatics.OpenLevel` "Level01")
    (else
      (`/Engine/EditorBlueprintResources/StandardMacros.IsValid` _nextcheckpoint
        (:`Is Valid`
          (bind _asbp_checkpoint (cast `/Game/Blueprints/BP_Checkpoint` _nextcheckpoint))
          (set `/Game/Blueprints/BP_Checkpoint.CanStart` true _asbp_checkpoint)
          (bind _ghost (`/Game/Blueprints/BP_Checkpoint.Ghost` _asbp_checkpoint))
          (`/Engine/EditorBlueprintResources/StandardMacros.IsValid` _ghost
            (:`Is Valid`
              (`self.SetActorHiddenInGame` _ghost false)
              (bind _returnvalue (`GameplayStatics.GetActorOfClass` "/Game/Blueprints/BP_TutorialArrow.BP_TutorialArrow_C"))
              (`/Engine/EditorBlueprintResources/StandardMacros.IsValid` _returnvalue
                (:`Is Valid`
                  (bind _ghost_2 (`/Game/Blueprints/BP_Checkpoint.Ghost` _asbp_checkpoint))
                  (`/Engine/EditorBlueprintResources/StandardMacros.IsValid` _ghost_2
                    (:`Is Valid`
                      (set `/Game/Blueprints/BP_TutorialArrow.CurrentTarget` _ghost_2 _returnvalue))))))))))))

(event `self.Box.OnComponentEndOverlap`
  (params (OverlappedComponent :type "PrimitiveComponent Object Reference") (OtherActor :type "Actor Object Reference") (OtherComp :type "PrimitiveComponent Object Reference") (OtherBodyIndex :type Integer))
  (bind _ghost (`self.Ghost`))
  (cast `/Game/Blueprints/BP_PlayerCharacter` OtherActor)
  (`/Engine/EditorBlueprintResources/StandardMacros.IsValid` _ghost
    (:`Is Valid`
      (bind _asbp_ghost (cast `/Game/Blueprints/BP_Ghost` _ghost))
      (if (`/Game/Blueprints/BP_Ghost.Completed` _asbp_ghost)
        (if (`/Game/Blueprints/BP_Ghost.IsAutoDisappear` _asbp_ghost)
          (`/Game/Blueprints/BP_Ghost.CompleteGhost` _asbp_ghost))))))

(fn `SetText`
  (bind _ghost (`self.Ghost`))
  (`/Engine/EditorBlueprintResources/StandardMacros.IsValid` _ghost
    (:`Is Valid`
      (bind _asbp_ghost (cast `/Game/Blueprints/BP_Ghost` _ghost))
      (bind _asbpw_text (cast `/Game/UI/BPW_Text` (`WidgetComponent.GetUserWidgetObject` (`/Game/Blueprints/BP_Ghost.TextWidget` _asbp_ghost))))
      (set `/Game/UI/BPW_Text.text` (`KismetTextLibrary.Conv_StringToText` (`|GetArrayItem` (`self.TextArray`) (`self.CurrentIndex`))) _asbpw_text))))

(fn `UserConstructionScript`)