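; Enemy AI controller that runs BT_Enemy and feeds its blackboard with target and combat data.
; Perception of actors tagged Friendly or Zombie sets them as the enemy with line of sight, while other updates start a timer that later clears both.
; On possess it records the start location and, after a delay for weapon spawning, copies an armed villager's weapon range into the blackboard.
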(event `self.AIPerception.OnTargetPerceptionUpdated`
  (params (Actor :type "Actor Object Reference") (Stimulus :type "AIStimulus Structure"))
  (bind _blackboard (`self.Blackboard`))
  (if (and (or (`self.ActorHasTag` Actor "Friendly") (`self.ActorHasTag` Actor "Zombie")) (`.bSuccessfullySensed` (break `AIStimulus` Stimulus)))
    (`KismetSystemLibrary.K2_ClearAndInvalidateTimerHandle` (`self.EnemyTimer`))
    (`BlackboardComponent.SetValueAsBool` _blackboard (`self.HasLineOfSight`) true)
    (`BlackboardComponent.SetValueAsObject` _blackboard (`self.EnemyActor`) Actor)
    (else
      (bind _returnvalue (`KismetSystemLibrary.K2_SetTimerDelegate` (delegate `StartEnemyTimer`) (`self.LineOfSightTimer`)))
      (set `self.EnemyTimer` _returnvalue))))

(event `StartEnemyTimer`
  (bind _blackboard (`self.Blackboard`))
  (`BlackboardComponent.SetValueAsBool` _blackboard (`self.HasLineOfSight`) false)
  (`BlackboardComponent.SetValueAsObject` _blackboard (`self.EnemyActor`) null))

(event `self.ReceivePossess`
  (params (PossessedPawn :type "Pawn Object Reference"))
  (bind _blackboard (`self.Blackboard`))
  (`self.RunBehaviorTree` "/Game/Blueprints/BT_Enemy.BT_Enemy")
  (`BlackboardComponent.SetValueAsVector` _blackboard (`self.Start Location`) (`self.K2_GetActorLocation` (`self.K2_GetPawn`)))
  ;[1 1 1] Need a delay so weapon is spawned in
  (`KismetSystemLibrary.Delay` 1.0)
  (bind _asbp_armed_villager (cast `/Game/Blueprints/BP_ArmedVillager` (`self.K2_GetPawn`)))
  (bind _currentweapon (`/Game/Blueprints/BP_ArmedVillager.CurrentWeapon` _asbp_armed_villager))
  (`/Engine/EditorBlueprintResources/StandardMacros.IsValid` _currentweapon
    (:`Is Valid`
      (`BlackboardComponent.SetValueAsFloat` _blackboard (`self.Range`) (`/Game/Blueprints/BP_BaseWeapon.Range` _currentweapon)))))

(fn `UserConstructionScript`)