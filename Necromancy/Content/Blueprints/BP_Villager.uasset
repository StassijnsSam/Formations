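; Villager character that fights zombies and friendlies, becomes a scoring physics corpse when killed, and can be raised as an AI-controlled zombie.
; Raise swaps tags, material and controller and resets health; a raised villager fights enemies and is destroyed on death.
; DamageZone overlaps track targets for timed attacks on BPC_Health, whose events drive the health bar and hit flash.
; As a zombie, PushZone launches MoveableLevel objects, scoring their mass when first dislodged.
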(event `self.PushZone.OnComponentBeginOverlap`
  (params (OverlappedComponent :type "PrimitiveComponent Object Reference") (OtherActor :type "Actor Object Reference") (OtherComp :type "PrimitiveComponent Object Reference") (OtherBodyIndex :type Integer) (bFromSweep :type Boolean) (SweepResult :type "HitResult Structure (by ref)"))
  (bind (_returnvalue_x _returnvalue_y) (`KismetMathLibrary.BreakVector` (* (`KismetMathLibrary.Normal` (- (`self.K2_GetActorLocation` OtherActor) (`self.K2_GetActorLocation`))) 1000.0)))
  (if (`self.ActorHasTag` "Zombie")
    (if (`self.ActorHasTag` OtherActor "MoveableLevel")
      (if (not (`SceneComponent.IsSimulatingPhysics` OtherComp "None"))
        (bind _asbp_my_game_mode (cast `/Game/Blueprints/BP_MyGameMode` (`GameplayStatics.GetGameMode`)))
        (`PrimitiveComponent.SetSimulatePhysics` OtherComp true)
        (`/Game/Blueprints/BP_MyGameMode.IncrementScore` _asbp_my_game_mode (`KismetMathLibrary.FCeil` (`PrimitiveComponent.GetMass` OtherComp))))
      (`PrimitiveComponent.AddImpulse` OtherComp (`KismetMathLibrary.MakeVector` _returnvalue_x _returnvalue_y 1000.0) "None" false))))

(event `self.BPC_Health.OnDamage`
  (bind _asbpw_enemy_health_bar (cast `/Game/UI/BPW_EnemyHealthBar` (`WidgetComponent.GetUserWidgetObject` (`self.Health Bar`))))
  (set `/Game/UI/BPW_EnemyHealthBar.HealthPercentage` (`/Game/Blueprints/BPC_Health.GetHealthPercentage` (`self.BPC_Health`)) _asbpw_enemy_health_bar)
  (`PrimitiveComponent.SetMaterial` (`self.Capsule`) 0 "/Game/StarterContent/Materials/M_Basic_Floor.M_Basic_Floor")
  (`KismetSystemLibrary.Delay` 0.1)
  (`PrimitiveComponent.SetMaterial` (`self.Capsule`) 0 (`self.OriginalMaterial`)))

(event `self.ReceiveBeginPlay`
  (bind _bpc_health (`self.BPC_Health`))
  (`parent.ReceiveBeginPlay`)
  (set `self.OriginalMaterial` (`PrimitiveComponent.GetMaterial` (`self.Capsule`) 0))
  (if (`self.isDeadFromStart`)
    (set `self.ScoreOnKill` 0)
    ;[1 1 1] Kill the enemy
    (`/Game/Blueprints/BPC_Health.Do Damage` _bpc_health (`/Game/Blueprints/BPC_Health.CurrentHealth` _bpc_health))))

(event `self.BPC_Health.OnDead`
  ;[1 1 1] If a raised enemy dies its dead for good
  (if (`self.IsRaised`)
    (for _array_element (`self.GetAttachedActors` self true)
      (bind _asbp_move_target (cast `/Game/Blueprints/BP_MoveTarget` _array_element))
      (`self.K2_DestroyActor` _asbp_move_target))
    (`self.K2_DestroyActor`)
    (else
      ;[1 1 1] get rid of controller
      ; This is needed instead of unpossess since otherwise the old controller can not be deleted
      (`self.DetachFromControllerPendingDestroy`)
      ;[1 1 1] Set tag to Dead
      (set `self.Tags` (`self.DeadTag`))
      ;[1 1 1] Give enemy the dead material
      (`self.ChangeMaterial` "/Game/Materials/MI_Dead.MI_Dead")
      ;[1 1 1] Simulate physics on dead body
      (set `self.OriginalMaterial` "/Game/Materials/MI_Dead.MI_Dead")
      (`PrimitiveComponent.SetSimulatePhysics` (`self.CapsuleComponent`) true)
      (bind _asbpw_enemy_health_bar (cast `/Game/UI/BPW_EnemyHealthBar` (`WidgetComponent.GetUserWidgetObject` (`self.Health Bar`))))
      (set `/Game/UI/BPW_EnemyHealthBar.HealthPercentage` (`/Game/Blueprints/BPC_Health.GetHealthPercentage` (`self.BPC_Health`)) _asbpw_enemy_health_bar)
      (bind _asbp_my_game_mode (cast `/Game/Blueprints/BP_MyGameMode` (`GameplayStatics.GetGameMode`)))
      (`/Game/Blueprints/BP_MyGameMode.IncrementScore` _asbp_my_game_mode (`self.ScoreOnKill`)))))

(event `self.DamageZone.OnComponentBeginOverlap`
  (params (OverlappedComponent :type "PrimitiveComponent Object Reference") (OtherActor :type "Actor Object Reference") (OtherComp :type "PrimitiveComponent Object Reference") (OtherBodyIndex :type Integer) (bFromSweep :type Boolean) (SweepResult :type "HitResult Structure (by ref)"))
  (`/Engine/EditorBlueprintResources/StandardMacros.IsValid` OtherActor
    (:`Is Valid`
      (`|ExecutionSequence`
        (:`then_0`
          (if (or (`/Game/Blueprints/BPC_Health.IsDead` (`self.BPC_Health`)) (`self.ActorHasTag` OtherActor "Dead"))
            _
            (elif (`self.IsRaised`)
              (if (`self.ActorHasTag` OtherActor "Enemy")
                (`KismetArrayLibrary.Array_AddUnique` (`self.NearbyEnemies`) OtherActor :!label _label)
                (set `self.CurrentEnemy` (`|GetArrayItem` (`self.NearbyEnemies`)))
                (`/Engine/EditorBlueprintResources/StandardMacros.IsValid` (`self.CurrentEnemy`)
                  (:`Is Valid`
                    _)
                  (:`Is Not Valid`
                    (set `self.CurrentEnemy` OtherActor)))
                (`KismetSystemLibrary.K2_SetTimerDelegate` (delegate `DamageCurrentEnemyTarget`) (`self.AttackInterval`) true))
              (elif (or (`self.ActorHasTag` OtherActor "Zombie") (`self.ActorHasTag` OtherActor "Friendly"))
                (goto _label)))))))))

(event `DamageCurrentEnemyTarget`
  (bind _nearbyenemies (`self.NearbyEnemies`))
  (bind _currentenemy (`self.CurrentEnemy`))
  (bind _currentenemy_2 (`self.CurrentEnemy`))
  (bind _returnvalue (`self.GetComponentByClass` _currentenemy_2 "/Game/Blueprints/BPC_Health.BPC_Health_C"))
  (`/Engine/EditorBlueprintResources/StandardMacros.IsValid` _currentenemy_2
    (:`Is Valid`
      (`/Engine/EditorBlueprintResources/StandardMacros.IsValid` _returnvalue
        (:`Is Valid`
          (if (`/Game/Blueprints/BPC_Health.IsDead` (`self.BPC_Health`))
            (`/Engine/EditorBlueprintResources/StandardMacros.IsValid` _currentenemy :!label _label_2
              (:`Is Valid`
                (`KismetArrayLibrary.Array_RemoveItem` (`self.NearbyEnemies`) _currentenemy)
                (`KismetSystemLibrary.K2_ClearTimer` null "DamageCurrentEnemyTarget")
                (if (> (`KismetArrayLibrary.Array_Length` _nearbyenemies) 0)
                  (set `self.CurrentEnemy` (`|GetArrayItem` _nearbyenemies))
                  (else
                    (set `self.CurrentEnemy` null)))))
            (else
              (bind _iskilled (message `/Game/Blueprints/BPI_Damageable.Do Damage` _returnvalue (`self.DamageAmount`)))
              (if _iskilled
                (goto _label_2)))))))))

(event `self.DamageZone.OnComponentEndOverlap`
  (params (OverlappedComponent :type "PrimitiveComponent Object Reference") (OtherActor :type "Actor Object Reference") (OtherComp :type "PrimitiveComponent Object Reference") (OtherBodyIndex :type Integer))
  (bind _nearbyenemies (`self.NearbyEnemies`))
  (`/Engine/EditorBlueprintResources/StandardMacros.IsValid` OtherActor
    (:`Is Valid`
      (if (`KismetArrayLibrary.Array_Contains` (`self.NearbyEnemies`) OtherActor)
        (`KismetArrayLibrary.Array_RemoveItem` (`self.NearbyEnemies`) OtherActor)
        (if (== OtherActor (`self.CurrentEnemy`))
          (`KismetSystemLibrary.K2_ClearTimer` null "DamageCurrentEnemyTarget")
          (if (> (`KismetArrayLibrary.Array_Length` _nearbyenemies) 0)
            (set `self.CurrentEnemy` (`|GetArrayItem` _nearbyenemies))
            (else
              (set `self.CurrentEnemy` null))))))))

(fn `ChangeMaterial`
  (params (Material :type "MaterialInstance Object Reference"))
  (`PrimitiveComponent.SetMaterial` (`self.RightHand`) 0 Material)
  (`PrimitiveComponent.SetMaterial` (`self.LeftHand`) 0 Material)
  (`PrimitiveComponent.SetMaterial` (`self.Capsule`) 0 Material))

(fn `Raise`
  (locals (newTags :type "Array of Name") (ZombieAIClass :type "Actor Class Reference" :default "BlueprintGeneratedClass'/Game/Blueprints/BP_ZombieAIController.BP_ZombieAIController_C'"))
  (bind (_returnvalue_location _returnvalue_rotation) (`KismetMathLibrary.BreakTransform` (`self.GetTransform` (`GameplayStatics.GetPlayerPawn` 0))))
  (`self.ChangeMaterial` "/Game/Materials/MI_Zombie.MI_Zombie")
  (set `self.OriginalMaterial` "/Game/Materials/MI_Zombie.MI_Zombie")
  (set `self.Tags` (`local.newTags`))
  (set `self.IsRaised` true)
  (`PrimitiveComponent.SetSimulatePhysics` (`self.CapsuleComponent`) false)
  (`self.K2_SetActorRotation` _returnvalue_rotation)
  (`/Game/Blueprints/BPC_Health.ResetHealth` (`self.BPC_Health`))
  (bind _returnvalue (`|SpawnActorFromClass` (`local.ZombieAIClass`) (`KismetMathLibrary.MakeTransform` (0.0 0.0 0.0)) "Undefined" "OverrideRootScale" null null))
  (bind _asbp_zombie_aicontroller (cast `/Game/Blueprints/BP_ZombieAIController` _returnvalue))
  (`Controller.Possess` _asbp_zombie_aicontroller self))

(fn `UpdateWalkSpeed`
  (params (WalkSpeed :type "Float (double-precision)"))
  (set `CharacterMovementComponent.MaxWalkSpeed` WalkSpeed (`self.CharacterMovement`)))

(fn `UserConstructionScript`
  (`parent.UserConstructionScript`)
  (if (`self.isDeadFromStart`)
    (`self.ChangeMaterial` "/Game/Materials/MI_Dead.MI_Dead")))