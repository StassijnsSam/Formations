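; BP_TutorialArrow is a tutorial pointer actor that follows its owner and points toward a target actor.
; On BeginPlay it falls back to the first player pawn if no valid owner is set, then teleports to and attaches to that owner.
; Each Tick it sets its rotation to look from the owner's location toward CurrentTarget, when both are valid.
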(event `self.ReceiveBeginPlay`
  (bind _currentowner (`self.CurrentOwner`))
  (`/Engine/EditorBlueprintResources/StandardMacros.IsValid` _currentowner
    (:`Is Valid`
      _)
    (:`Is Not Valid`
      (set `self.CurrentOwner` (`GameplayStatics.GetPlayerPawn` 0))))
  (`self.K2_SetActorLocation` (`self.K2_GetActorLocation` _currentowner) false true)
  (`self.K2_AttachToActor` _currentowner "None" "SnapToTarget" "KeepRelative" "KeepRelative"))

(event `self.ReceiveTick`
  (params (DeltaSeconds :type "Float (single-precision)"))
  (bind _currenttarget (`self.CurrentTarget`))
  (bind _currentowner (`self.CurrentOwner`))
  (`/Engine/EditorBlueprintResources/StandardMacros.IsValid` _currenttarget
    (:`Is Valid`
      (`/Engine/EditorBlueprintResources/StandardMacros.IsValid` _currentowner
        (:`Is Valid`
          (`self.K2_SetActorRotation` (`KismetMathLibrary.FindLookAtRotation` (`self.K2_GetActorLocation` _currentowner) (`self.K2_GetActorLocation` _currenttarget))))))))

(fn `UserConstructionScript`)